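; Game mode for a fighting match between a player and an AI opponent, running intro, round timer and game over.
; BeginPlay spawns and possesses both fighters from GameInstance classes, cross-links them, sets camera and HUD, then freezes both until the intro timer ends.
; Tick counts down with Delay and shows game over after a knockout.
; On timeout, unequal health always zeroes Player 2, even when Player 1 trails; ties zero both.
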(event Custom|OnCountdownFinished
  (bind _assfiigameinstance (Utilities|Casting|CastToSFIIGameinstance (Game|GetGameInstance)))
  (Utilities|FlowControl|DoOnce false
    (:Completed
      (Input|EnableInput (Variables|/Game/SFIIGameinstance.SFIIGameinstance_C|GetPlayer1Character _assfiigameinstance) (Variables|/Game/SFIIGameinstance.SFIIGameinstance_C|GetPlayer1Controller _assfiigameinstance))
      (AI|Logic|StartLogic (Variables|/Script/AIModule.AIController|GetBrainComponent (Variables|/Game/SFIIGameinstance.SFIIGameinstance_C|GetPlayer2Controller _assfiigameinstance)))
      (Variables|Default|SetbRoundStart true))))

(event EventBeginPlay
  (bind _returnvalue (Game|GetGameInstance))
  (bind _returnvalue_2 (Game|GetPlayerController 0))
  (Utilities|FlowControl|Sequence
    (:then_0
      (bind _assfiigameinstance (Utilities|Casting|CastToSFIIGameinstance (Game|GetGameInstance)))
      (bind _returnvalue_3 (Game|SpawnActorfromClass (Variables|/Game/SFIIGameinstance.SFIIGameinstance_C|GetPlayer1CharacterClass _assfiigameinstance) (Transformation|GetActorTransform (Class|GameModeBase|FindPlayerStart 0 "Player1")) "AdjustIfPossibleButAlwaysSpawn" 0 0))
      (bind _assfiigameinstance_2 (Utilities|Casting|CastToSFIIGameinstance _returnvalue))
      (bind _output_get (Variables|/Game/SFIIGameinstance.SFIIGameinstance_C|SetPlayer1Controller _assfiigameinstance_2 (Game|GetPlayerController 0)))
      (bind _output_get_2 (Variables|/Game/SFIIGameinstance.SFIIGameinstance_C|SetPlayer1Character _assfiigameinstance_2 _returnvalue_3))
      (Pawn|Possess _output_get _output_get_2))
    (:then_1
      (bind _returnvalue_4 (Game|SpawnActorfromClass (Variables|/Game/SFIIGameinstance.SFIIGameinstance_C|GetPlayer2CharacterClass _assfiigameinstance) (Transformation|GetActorTransform (Class|GameModeBase|FindPlayerStart 0 "Player2")) "AdjustIfPossibleButAlwaysSpawn" 0 0))
      (bind _assfiigameinstance_3 (Utilities|Casting|CastToSFIIGameinstance _returnvalue))
      (bind _output_get_3 (Variables|/Game/SFIIGameinstance.SFIIGameinstance_C|SetPlayer2Controller _assfiigameinstance_3 (AI|GetAIController _returnvalue_4)))
      (bind _output_get_4 (Variables|/Game/SFIIGameinstance.SFIIGameinstance_C|SetPlayer2Character _assfiigameinstance_3 _returnvalue_4))
      (Pawn|Possess _output_get_3 _output_get_4))
    (:then_2
      (bind _assfiigameinstance_4 (Utilities|Casting|CastToSFIIGameinstance (Game|GetGameInstance)))
      (bind _output_get_5 (Variables|/Script/SFII.SFIICharacter|SetOtherPlayer (Variables|/Game/SFIIGameinstance.SFIIGameinstance_C|GetPlayer1Character _assfiigameinstance_4) (Variables|/Game/SFIIGameinstance.SFIIGameinstance_C|GetPlayer2Character _assfiigameinstance_4)))
      (Variables|/Script/SFII.SFIICharacter|SetOtherPlayer _output_get_5 (Variables|/Game/SFIIGameinstance.SFIIGameinstance_C|GetPlayer1Character _assfiigameinstance_4)))
    (:then_3
      (Game|Player|SetViewTargetwithBlend (Game|GetPlayerController 0) (Variables|Default|GetCamera) 0.0 "VTBlend_Linear" 0.0 false)
      (bind _returnvalue_5 (UserInterface|CreateWidget "/Game/Gameplay/WBP_Gameplay.WBP_Gameplay_C"))
      (UserInterface|Viewport|AddtoViewport _returnvalue_5 0))
    (:then_4
      (Input|SetInputModeGameOnly _returnvalue_2)
      (bind _assfiigameinstance_5 (Utilities|Casting|CastToSFIIGameinstance (Game|GetGameInstance)))
      (Input|DisableInput (Variables|/Game/SFIIGameinstance.SFIIGameinstance_C|GetPlayer1Character _assfiigameinstance_5) _returnvalue_2)
      (AI|Logic|StopLogic (Variables|/Script/AIModule.AIController|GetBrainComponent (Variables|/Game/SFIIGameinstance.SFIIGameinstance_C|GetPlayer2Controller _assfiigameinstance_5)) "")
      (Utilities|Time|SetTimerbyEvent (delegate Custom|OnCountdownFinished) (Variables|Default|GetIntroTime)))))

(event EventTick
  (params (DeltaSeconds :type Float%20%28single-precision%29))
  (if (Variables|Default|GetbRoundStart)
    (bind _assfiigameinstance (Utilities|Casting|CastToSFIIGameinstance (Game|GetGameInstance)))
    (if (or (== (Variables|/Script/SFII.SFIICharacter|GetCurrentHealth (Variables|/Game/SFIIGameinstance.SFIIGameinstance_C|GetPlayer1Character _assfiigameinstance)) 0.0) (== (Variables|/Script/SFII.SFIICharacter|GetCurrentHealth (Variables|/Game/SFIIGameinstance.SFIIGameinstance_C|GetPlayer2Character _assfiigameinstance)) 0.0))
      (Utilities|FlowControl|DoOnce false
        (:Completed
          (Utilities|FlowControl|Delay (Variables|Default|GetEndOfRoundDelay))
          (bind _returnvalue (UserInterface|CreateWidget "/Game/Gameplay/WBP_GameOver.WBP_GameOver_C"))
          (UserInterface|Viewport|AddtoViewport _returnvalue 0)))
      (elif (== (Variables|Default|GetRoundTime) 0.0)
        (Utilities|FlowControl|DoOnce false
          (:Completed
            (bind _assfiigameinstance_2 (Utilities|Casting|CastToSFIIGameinstance (Game|GetGameInstance)))
            (if (> (Variables|/Script/SFII.SFIICharacter|GetCurrentHealth (Variables|/Game/SFIIGameinstance.SFIIGameinstance_C|GetPlayer1Character _assfiigameinstance_2)) (Variables|/Script/SFII.SFIICharacter|GetCurrentHealth (Variables|/Game/SFIIGameinstance.SFIIGameinstance_C|GetPlayer2Character _assfiigameinstance_2)))
              ;[1 1 1] Player 2 Timed Out
              (Utilities|FlowControl|DoOnce false
                (:Completed
                  (Variables|/Script/SFII.SFIICharacter|SetCurrentHealth (Variables|/Game/SFIIGameinstance.SFIIGameinstance_C|GetPlayer2Character _assfiigameinstance_2) 0.0)
                  (Class|SFIICharacter|UpdateHealth (Variables|/Game/SFIIGameinstance.SFIIGameinstance_C|GetPlayer2Character _assfiigameinstance_2) 0.0 "HIGH")))
              (elif (> (Variables|/Script/SFII.SFIICharacter|GetCurrentHealth (Variables|/Game/SFIIGameinstance.SFIIGameinstance_C|GetPlayer2Character _assfiigameinstance_2)) (Variables|/Script/SFII.SFIICharacter|GetCurrentHealth (Variables|/Game/SFIIGameinstance.SFIIGameinstance_C|GetPlayer1Character _assfiigameinstance_2)))
                ;[1 1 1] Player 1 Timed Out
                (Utilities|FlowControl|DoOnce false
                  (:Completed
                    (Variables|/Script/SFII.SFIICharacter|SetCurrentHealth (Variables|/Game/SFIIGameinstance.SFIIGameinstance_C|GetPlayer2Character _assfiigameinstance_2) 0.0)
                    (Class|SFIICharacter|UpdateHealth (Variables|/Game/SFIIGameinstance.SFIIGameinstance_C|GetPlayer2Character _assfiigameinstance_2) 0.0 "HIGH")))
                (else
                  ;[1 1 1] Both Players Timed out
                  (Utilities|FlowControl|DoOnce false
                    (:Completed
                      (bind _output_get (Variables|/Script/SFII.SFIICharacter|SetCurrentHealth (Variables|/Game/SFIIGameinstance.SFIIGameinstance_C|GetPlayer1Character _assfiigameinstance_2) 0.0))
                      (Variables|/Script/SFII.SFIICharacter|SetCurrentHealth (Variables|/Game/SFIIGameinstance.SFIIGameinstance_C|GetPlayer2Character _assfiigameinstance_2) _output_get)
                      (Class|SFIICharacter|UpdateHealth (Variables|/Game/SFIIGameinstance.SFIIGameinstance_C|GetPlayer1Character _assfiigameinstance_2) 0.0 "HIGH")
                      (Class|SFIICharacter|UpdateHealth (Variables|/Game/SFIIGameinstance.SFIIGameinstance_C|GetPlayer2Character _assfiigameinstance_2) 0.0 "HIGH"))))))))
        (else
          ;[1 1 1] Decrement Round Time
          (Utilities|FlowControl|Delay 1.0)
          (Math|Float|DecrementFloat (Variables|Default|GetRoundTime)))))))

(fn ConstructionScript)